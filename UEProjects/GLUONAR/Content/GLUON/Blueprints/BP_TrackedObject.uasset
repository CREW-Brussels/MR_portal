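; BP_TrackedObject is an AR actor that shows debug feedback for tracked geometry once an image is detected.
; Each Tick checks for any ARTrackedImage, then prints the name of the first entry from the unfiltered list of all geometries and draws its debug outline.
; A node to move the actor's root to that geometry's transform is present but unconnected, so the actor does not follow it.
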(event `self.ReceiveTick`
  (params (DeltaSeconds :type "Float (single-precision)"))
  (bind _returnvalue (`ARBlueprintLibrary.GetAllGeometriesByClass` "/Script/AugmentedReality.ARTrackedImage"))
  (if (> (`KismetArrayLibrary.Array_Length` _returnvalue) 0)
    (bind _returnvalue_2 (`ARBlueprintLibrary.GetAllGeometries`))
    (bind _output (`|GetArrayItem` _returnvalue_2))
    (`KismetSystemLibrary.PrintString` (`KismetSystemLibrary.GetDisplayName` _output))
    (`ARBlueprintLibrary.DebugDrawTrackedGeometry` _output (struct :`R` 1.0 :`G` 1.0 :`A` 0.75) 1.0)))

(fn `UserConstructionScript`)